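; Player pawn for a grid-based item-fetching game, handling movement, pause menu, carried item and NPC dialogue.
; WASD moves one tile via timelines with input disabled, blocked by four collision boxes detecting CubeWall_BP.
; E finds NPCs or items by matching locations to pick up, drop, swap or talk, driving HUD text through staged clues.
; Satisfied NPCs are destroyed when conversation ends; five removals open the EndGame level.
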(event `Key|Escape`
  (params (Key :type "Key Structure"))
  (:`Released`
    (if (`self.Pause`)
      (bind _foundwidgets (`WidgetBlueprintLibrary.GetAllWidgetsOfClass` "/Game/MenuWidgets/PauseMenu.PauseMenu_C" false))
      (for _array_element _foundwidgets
        (`Widget.RemoveFromParent` _array_element)
        (set `self.Pause` false)
        (set `PlayerController.bShowMouseCursor` false (`GameplayStatics.GetPlayerController` 0)))
      (else
        (bind _returnvalue (`|CreateWidget` "/Game/MenuWidgets/PauseMenu.PauseMenu_C"))
        (`UserWidget.AddToViewport` _returnvalue 2)
        (set `self.Pause` true)
        (set `PlayerController.bShowMouseCursor` true (`GameplayStatics.GetPlayerController` 0))))))

(event `Key|E`
  (params (Key :type "Key Structure"))
  ;[1 1 1] Player Logic
  (:`Pressed`
    (bind _standingonitem (`self.Check if Standing on Class Member` "/Game/Characters/NPC_BP.NPC_BP_C"))
    (if _standingonitem
      (if (`/Game/BluePrints/HUD.In_Conversation` (`self.HUDReference`))
        (`self.EndCoversation`)
        (if (>= (`self.KillCounter`) 5)
          (`self.VictoryCondition`))
        (else
          (set `/Game/BluePrints/HUD.In_Conversation` true (`self.HUDReference`))
          (`self.StartConversation`)))
      (elif (== (`/Game/BluePrints/HUD.Item_Carried` (`self.HUDReference`)) 0)
        (`self.PickupItem`)
        (else
          (bind _standingonitem_2 (`self.Check if Standing on Class Member` "/Game/Inventory/Item_BP.Item_BP_C"))
          (if _standingonitem_2
            (`self.SwapItem` (`/Game/BluePrints/HUD.Item_Carried` (`self.HUDReference`)))
            (else
              (`self.DropItem`))))))))

(event `self.ReceiveBeginPlay`
  ;[1 1 1] CreateHUD
  (bind _returnvalue (`|CreateWidget` "/Game/BluePrints/HUD.HUD_C"))
  (bind _output_get (set `self.HUDReference` _returnvalue))
  (`UserWidget.AddToViewport` _output_get 0))

(event `Key|W`
  (params (Key :type "Key Structure"))
  ;[1 1 1] W Movement
  (:`Released`
    (if (`|GetArrayItem` (`self.Movement`) (`self.WKey`))
      _
      (elif (not (or (`/Game/BluePrints/HUD.In_Conversation` (`self.HUDReference`)) (`self.Pause`)))
        (`self.DisableInput` (`GameplayStatics.GetPlayerController` 0))
        (bind _output_get (set `self.TemporaryPosition` (`self.K2_GetActorLocation`)))
        (bind (_direction _newtrack_1) (`Timeline|Timeline_0` :!via `PlayFromStart`)
          (:`Update`
            (`self.K2_SetActorLocation` (`KismetMathLibrary.VLerp` _output_get (+ _output_get (0.0 100.0 0.0)) _newtrack_1)))
          (:`Finished`
            (`self.EnableInput` (`GameplayStatics.GetPlayerController` 0))))))))

(event `self.DCollBox.OnComponentBeginOverlap`
  (params (OverlappedComponent :type "PrimitiveComponent Object Reference") (OtherActor :type "Actor Object Reference") (OtherComp :type "PrimitiveComponent Object Reference") (OtherBodyIndex :type Integer) (bFromSweep :type Boolean) (SweepResult :type "HitResult Structure (by ref)"))
  ;[1 1 1] Collision Boxes Check
  (cast `/Game/BluePrints/CubeWall_BP` OtherActor)
  (`|VariableSetRef` (`|GetArrayItem` (`self.Movement`) (`self.DKey`)) true))

(event `self.DCollBox.OnComponentEndOverlap`
  (params (OverlappedComponent :type "PrimitiveComponent Object Reference") (OtherActor :type "Actor Object Reference") (OtherComp :type "PrimitiveComponent Object Reference") (OtherBodyIndex :type Integer))
  ;[1 1 1] Collision Boxes Check
  (cast `/Game/BluePrints/CubeWall_BP` OtherActor)
  (`|VariableSetRef` (`|GetArrayItem` (`self.Movement`) (`self.DKey`))))

(event `self.WCollBox.OnComponentBeginOverlap`
  (params (OverlappedComponent :type "PrimitiveComponent Object Reference") (OtherActor :type "Actor Object Reference") (OtherComp :type "PrimitiveComponent Object Reference") (OtherBodyIndex :type Integer) (bFromSweep :type Boolean) (SweepResult :type "HitResult Structure (by ref)"))
  ;[1 1 1] Collision Boxes Check
  (cast `/Game/BluePrints/CubeWall_BP` OtherActor)
  (`|VariableSetRef` (`|GetArrayItem` (`self.Movement`) (`self.WKey`)) true))

(event `Key|S`
  (params (Key :type "Key Structure"))
  ;[1 1 1] S Movement
  (:`Released`
    (if (`|GetArrayItem` (`self.Movement`) (`self.SKey`))
      _
      (elif (not (or (`/Game/BluePrints/HUD.In_Conversation` (`self.HUDReference`)) (`self.Pause`)))
        (`self.DisableInput` (`GameplayStatics.GetPlayerController` 0))
        (bind _output_get (set `self.TemporaryPosition` (`self.K2_GetActorLocation`)))
        (bind (_direction _newtrack_1) (`Timeline|Timeline_1` :!via `PlayFromStart`)
          (:`Update`
            (`self.K2_SetActorLocation` (`KismetMathLibrary.VLerp` _output_get (+ _output_get (0.0 -100.0 0.0)) _newtrack_1)))
          (:`Finished`
            (`self.EnableInput` (`GameplayStatics.GetPlayerController` 0))))))))

(event `self.WCollBox.OnComponentEndOverlap`
  (params (OverlappedComponent :type "PrimitiveComponent Object Reference") (OtherActor :type "Actor Object Reference") (OtherComp :type "PrimitiveComponent Object Reference") (OtherBodyIndex :type Integer))
  ;[1 1 1] Collision Boxes Check
  (cast `/Game/BluePrints/CubeWall_BP` OtherActor)
  (`|VariableSetRef` (`|GetArrayItem` (`self.Movement`) (`self.WKey`))))

(event `self.SCollBox.OnComponentBeginOverlap`
  (params (OverlappedComponent :type "PrimitiveComponent Object Reference") (OtherActor :type "Actor Object Reference") (OtherComp :type "PrimitiveComponent Object Reference") (OtherBodyIndex :type Integer) (bFromSweep :type Boolean) (SweepResult :type "HitResult Structure (by ref)"))
  ;[1 1 1] Collision Boxes Check
  (cast `/Game/BluePrints/CubeWall_BP` OtherActor)
  (`|VariableSetRef` (`|GetArrayItem` (`self.Movement`) (`self.SKey`)) true))

(event `Key|A`
  (params (Key :type "Key Structure"))
  ;[1 1 1] A Movement
  (:`Released`
    (if (`|GetArrayItem` (`self.Movement`) (`self.AKey`))
      _
      (elif (not (or (`/Game/BluePrints/HUD.In_Conversation` (`self.HUDReference`)) (`self.Pause`)))
        (`self.DisableInput` (`GameplayStatics.GetPlayerController` 0))
        (bind _output_get (set `self.TemporaryPosition` (`self.K2_GetActorLocation`)))
        (bind (_direction _newtrack_1) (`Timeline|Timeline_2` :!via `PlayFromStart`)
          (:`Update`
            (`self.K2_SetActorLocation` (`KismetMathLibrary.VLerp` _output_get (+ _output_get (100.0 0.0 0.0)) _newtrack_1)))
          (:`Finished`
            (`self.EnableInput` (`GameplayStatics.GetPlayerController` 0))))))))

(event `self.SCollBox.OnComponentEndOverlap`
  (params (OverlappedComponent :type "PrimitiveComponent Object Reference") (OtherActor :type "Actor Object Reference") (OtherComp :type "PrimitiveComponent Object Reference") (OtherBodyIndex :type Integer))
  ;[1 1 1] Collision Boxes Check
  (cast `/Game/BluePrints/CubeWall_BP` OtherActor)
  (`|VariableSetRef` (`|GetArrayItem` (`self.Movement`) (`self.SKey`))))

(event `Key|D`
  (params (Key :type "Key Structure"))
  ;[1 1 1] D Movement
  (:`Released`
    (if (`|GetArrayItem` (`self.Movement`) (`self.DKey`))
      _
      (elif (not (or (`/Game/BluePrints/HUD.In_Conversation` (`self.HUDReference`)) (`self.Pause`)))
        (`self.DisableInput` (`GameplayStatics.GetPlayerController` 0))
        (bind _output_get (set `self.TemporaryPosition` (`self.K2_GetActorLocation`)))
        (bind (_direction _newtrack_1) (`Timeline|Timeline_3` :!via `PlayFromStart`)
          (:`Update`
            (`self.K2_SetActorLocation` (`KismetMathLibrary.VLerp` _output_get (+ _output_get (-100.0 0.0 0.0)) _newtrack_1)))
          (:`Finished`
            (`self.EnableInput` (`GameplayStatics.GetPlayerController` 0))))))))

(event `self.ACollBox.OnComponentBeginOverlap`
  (params (OverlappedComponent :type "PrimitiveComponent Object Reference") (OtherActor :type "Actor Object Reference") (OtherComp :type "PrimitiveComponent Object Reference") (OtherBodyIndex :type Integer) (bFromSweep :type Boolean) (SweepResult :type "HitResult Structure (by ref)"))
  ;[1 1 1] Collision Boxes Check
  (cast `/Game/BluePrints/CubeWall_BP` OtherActor)
  (`|VariableSetRef` (`|GetArrayItem` (`self.Movement`) (`self.AKey`)) true))

(event `self.ACollBox.OnComponentEndOverlap`
  (params (OverlappedComponent :type "PrimitiveComponent Object Reference") (OtherActor :type "Actor Object Reference") (OtherComp :type "PrimitiveComponent Object Reference") (OtherBodyIndex :type Integer))
  ;[1 1 1] Collision Boxes Check
  (cast `/Game/BluePrints/CubeWall_BP` OtherActor)
  (`|VariableSetRef` (`|GetArrayItem` (`self.Movement`) (`self.AKey`))))

(fn `Check if Standing on Class Member`
  (params (ActorClass :type "Actor Class Reference"))
  (returns (StandingOnItem :type Boolean))
  (bind _outactors (`GameplayStatics.GetAllActorsOfClass` ActorClass))
  (for _array_element _outactors
    (if (== (`self.K2_GetActorLocation` self) (`self.K2_GetActorLocation` _array_element) :`ErrorTolerance` 0.1)
      (return true)))
  (return false))

(fn `Conversation Give Clue`
  (params (HudRef :type "/Game/BluePrints/HUD Object Reference (by ref)") (Wanted :type "Integer (by ref)") (QStage :type "Integer (by ref)") (Actor :type "/Game/Characters/NPC_BP Object Reference (by ref)"))
  (for _index (range 4)
    (if (== QStage _index)
      (set `/Game/BluePrints/HUD.TextShow` (+ (* Wanted 10) _index) HudRef)
      (set `/Game/Characters/NPC_BP.QStage` (+ QStage 1) Actor)
      (return)))
  (set `/Game/BluePrints/HUD.TextShow` (+ (* Wanted 10) 4) HudRef))

(fn `Conversation Good Item`
  (params (HudRef :type "/Game/BluePrints/HUD Object Reference (by ref)") (ActorRef :type "/Game/Characters/NPC_BP Object Reference (by ref)") (MyItem :type "Integer (by ref)"))
  (set `/Game/BluePrints/HUD.TextShow` (+ (* MyItem 10) 5) HudRef)
  (set `/Game/BluePrints/HUD.Item_Carried` 0 HudRef)
  (set `/Game/Characters/NPC_BP.Item_Want` 0 ActorRef))

(fn `Conversation Progressing`
  (params (ItemCarriedReference :type "Integer (by ref)") (ItemWantReference :type "Integer (by ref)") (ConversationStage :type "Integer (by ref)") (HUDPassReference :type "/Game/BluePrints/HUD Object Reference (by ref)") (ActorPassRef :type "/Game/Characters/NPC_BP Object Reference (by ref)"))
  (locals (ItemCarried :type Integer) (ItemWant :type Integer) (ConversationStageReference :type Integer) (HudRef :type "/Game/BluePrints/HUD Object Reference") (ActorRef :type "/Game/Characters/NPC_BP Object Reference"))
  (bind _hudreference (`self.HUDReference`))
  (set `local.ItemCarried` ItemCarriedReference)
  (set `local.ItemWant` ItemWantReference)
  (set `local.ConversationStageReference` ConversationStage)
  (set `local.HudRef` _hudreference)
  (bind _output_get (set `local.ActorRef` ActorPassRef))
  (set `/Game/BluePrints/HUD.NPC_Face` (`/Game/Characters/NPC_BP.Identity` _output_get) _hudreference)
  (if (== (`local.ItemCarried`) (`local.ItemWant`))
    (`self.Conversation Good Item` (`local.HudRef`) (`local.ActorRef`) (`local.ItemWant`))
    (else
      (`self.Conversation Give Clue` (`local.HudRef`) (`local.ItemWant`) (`local.ConversationStageReference`) (`local.ActorRef`)))))

(fn `DropItem`
  (`|SpawnActorFromClass` "/Game/Inventory/Item_BP.Item_BP_C" (`KismetMathLibrary.MakeTransform` (`self.K2_GetActorLocation` self)) "Undefined" "OverrideRootScale" null (`/Game/BluePrints/HUD.Item_Carried` (`self.HUDReference`)) null)
  (set `/Game/BluePrints/HUD.Item_Carried` 0 (`self.HUDReference`)))

(fn `EndCoversation`
  (set `/Game/BluePrints/HUD.In_Conversation` false (`self.HUDReference`))
  (bind _outactors (`GameplayStatics.GetAllActorsOfClass` "/Game/Characters/NPC_BP.NPC_BP_C"))
  (for (_array_element _array_index) _outactors
    (if (== (`self.K2_GetActorLocation` self) (`self.K2_GetActorLocation` _array_element) :`ErrorTolerance` 0.1)
      (bind _output (`|GetArrayItem` _outactors _array_index))
      (if (== (`/Game/Characters/NPC_BP.Item_Want` _output) 0)
        (`self.K2_DestroyActor` _output)
        (bind _output_get (set `self.KillCounter` (+ (`self.KillCounter`) 1)))
        (`KismetSystemLibrary.PrintString` (`KismetStringLibrary.Conv_IntToString` _output_get))))))

(fn `PickupItem`
  (bind _outactors (`GameplayStatics.GetAllActorsOfClass` "/Game/Inventory/Item_BP.Item_BP_C"))
  (for (_array_element _array_index) _outactors
    (if (== (`self.K2_GetActorLocation` self) (`self.K2_GetActorLocation` _array_element) :`ErrorTolerance` 0.1)
      (bind _output (`|GetArrayItem` _outactors _array_index))
      (set `/Game/BluePrints/HUD.Item_Carried` (`/Game/Inventory/Item_BP.Index` _output) (`self.HUDReference`))
      (`self.K2_DestroyActor` _output))))

(fn `StartConversation`
  (bind _hudreference (`self.HUDReference`))
  (bind _outactors (`GameplayStatics.GetAllActorsOfClass` "/Game/Characters/NPC_BP.NPC_BP_C"))
  (for _array_element _outactors
    (if (== (`self.K2_GetActorLocation` self) (`self.K2_GetActorLocation` _array_element) :`ErrorTolerance` 0.1)
      (`self.Conversation Progressing` (`/Game/BluePrints/HUD.Item_Carried` _hudreference) (`/Game/Characters/NPC_BP.Item_Want` _array_element) (`/Game/Characters/NPC_BP.QStage` _array_element) _hudreference _array_element))))

(fn `SwapItem`
  (params (ItemCarried :type "Integer (by ref)"))
  (locals (TempCarriedItem :type Integer))
  (bind _output_get (set `local.TempCarriedItem` ItemCarried))
  (bind _outactors (`GameplayStatics.GetAllActorsOfClass` "/Game/Inventory/Item_BP.Item_BP_C"))
  (for (_array_element _array_index) _outactors
    (if (== (`self.K2_GetActorLocation` self) (`self.K2_GetActorLocation` _array_element) :`ErrorTolerance` 0.1)
      (bind _output (`|GetArrayItem` _outactors _array_index))
      (bind _output_get_2 (set `/Game/BluePrints/HUD.Item_Carried` (`/Game/Inventory/Item_BP.Index` _output) (`self.HUDReference`)))
      (`self.K2_DestroyActor` _output)
      (`|SpawnActorFromClass` "/Game/Inventory/Item_BP.Item_BP_C" (`KismetMathLibrary.MakeTransform` (`self.K2_GetActorLocation` self)) "Undefined" "OverrideRootScale" null _output_get null)
      (set `/Game/BluePrints/HUD.Item_Carried` _output_get_2 (`self.HUDReference`)))))

(fn `UserConstructionScript`)

(fn `VictoryCondition`
  (`GameplayStatics.OpenLevel` "EndGame"))