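; FloorA_BP is a floor piece whose appearance depends on whether it is flagged as a path.
; The construction script sets material slot 0 of its static mesh from the PathType array, using the IsPath boolean converted to an integer as the index.
; Both sides of the IsPath branch make the same call, so the index alone selects the material.
; The event graph has no runtime logic.
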(event `self.ReceiveBeginPlay`)

(fn `UserConstructionScript`
  (if (`self.IsPath`)
    (`PrimitiveComponent.SetMaterial` (`self.StaticMeshComponent`) 0 (`|GetArrayItem` (`self.PathType`) (`KismetMathLibrary.Conv_BoolToInt` (`self.IsPath`))))
    (else
      (`PrimitiveComponent.SetMaterial` (`self.StaticMeshComponent`) 0 (`|GetArrayItem` (`self.PathType`) (`KismetMathLibrary.Conv_BoolToInt` (`self.IsPath`)))))))