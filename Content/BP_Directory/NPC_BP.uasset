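; NPC_BP is an NPC Blueprint with a configurable appearance and dialog.
; The construction script builds a dynamic material from the NPCType entry selected by Identity, applies it to slot 0 of NPCModel, and passes DialogTrees to the DialogComponent.
; A SeenItemsLength helper returns the size of SeenItems.
; The OnInteract event is empty.
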(event `/Game/BP_Directory/InteractionInterface.OnInteract`
  (params (PlayerCharacter :type "Actor Object Reference") (ConversationStage :type Integer)))

(fn `SeenItemsLength`
  (returns (SeenItemLength :type Integer))
  (return (`BlueprintMapLibrary.Map_Length` (`self.SeenItems`))))

(fn `UserConstructionScript`
  (bind _npcmodel (`self.NPCModel`))
  (bind _returnvalue (`PrimitiveComponent.CreateDynamicMaterialInstance` _npcmodel 0 (`|GetArrayItem` (`self.NPCType`) (`self.Identity`)) "None"))
  (`PrimitiveComponent.SetMaterial` _npcmodel 0 _returnvalue)
  (set `/Game/Conversations/DialogComponent.DialogTree` (`self.DialogTrees`) (`self.DialogComponent`)))