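; Player Blueprint for an item-delivery game: swept axis movement with sprint, a pause menu, and a HUD widget that stores carried item and conversation state.
; E talks to a nearby NPC or picks up, drops or swaps items, using GetAllActorsOfClass location-tolerance scans.
; Dialogue sets a HUD text index from wanted item and clue stage.
; Satisfied NPCs are destroyed when conversation ends, and six removals open EndGame.
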(event `Key|E`
  (params (Key :type "Key Structure"))
  ;[1 1 1] Player Logic
  (:`Pressed`
    (bind _isstanding (`self.Check if Standing on Class Member` "/Game/BP_Directory/NPC_BP.NPC_BP_C"))
    (if _isstanding
      (if (`/Game/Widgets/HUD.In_Conversation` (`self.HUDReference`))
        (`self.EndCoversation`)
        (if (>= (`self.KillCounter`) 6)
          (`self.VictoryCondition`))
        (else
          (set `/Game/Widgets/HUD.In_Conversation` true (`self.HUDReference`))
          (`self.StartConversation`)))
      (elif (== (`/Game/Widgets/HUD.Item_Carried` (`self.HUDReference`)) 0)
        (`self.PickupItem`)
        (else
          (bind _isstanding_2 (`self.Check if Standing on Class Member` "/Game/BP_Directory/Item_BP.Item_BP_C"))
          (if _isstanding_2
            (`self.SwapItem` (`/Game/Widgets/HUD.Item_Carried` (`self.HUDReference`)))
            (else
              (`self.DropItem`))))))))

(event `self.ReceiveBeginPlay`
  ;[1 1 1] CreateHUD
  (bind _returnvalue (`|CreateWidget` "/Game/Widgets/HUD.HUD_C"))
  (bind _output_get (set `self.HUDReference` _returnvalue))
  (`UserWidget.AddToViewport` _output_get 0))

(event `InputAction|Exit`
  (params (Key :type "Key Structure"))
  ;[1 1 1] PauseMenu
  (:`Released`
    (if (`self.Pause`)
      (bind _foundwidgets (`WidgetBlueprintLibrary.GetAllWidgetsOfClass` "/Game/Widgets/PauseMenu.PauseMenu_C" false))
      (for _array_element _foundwidgets
        (`Widget.RemoveFromParent` _array_element)
        (bind _output_get (set `/Game/Widgets/PauseMenu.PauseState` false _array_element))
        (bind _output_get_2 (set `PlayerController.bShowMouseCursor` _output_get (`GameplayStatics.GetPlayerController` 0)))
        (set `self.Pause` _output_get_2))
      (else
        (bind _returnvalue (`|CreateWidget` "/Game/Widgets/PauseMenu.PauseMenu_C"))
        (`UserWidget.AddToViewport` _returnvalue 2)
        (bind _output_get_3 (set `/Game/Widgets/PauseMenu.PauseState` true _returnvalue))
        (bind _output_get_4 (set `PlayerController.bShowMouseCursor` _output_get_3 (`GameplayStatics.GetPlayerController` 0)))
        (set `self.Pause` _output_get_4)))))

(event `InputAxis|MoveRight`
  (params (AxisValue :type "Float (single-precision)"))
  ;[1 1 1] X Movement
  (if (!= AxisValue 0.0)
    (if (not (or (`/Game/Widgets/HUD.In_Conversation` (`self.HUDReference`)) (`self.Pause`)))
      (bind _output_get (set `self.TemporaryPosition` (`self.K2_GetActorLocation`)))
      (`self.K2_SetActorLocation` (+ _output_get (`KismetMathLibrary.MakeVector` (* (* AxisValue (`self.Speed`)) -1.0))) true))))

(event `InputAxis|MoveForward`
  (params (AxisValue :type "Float (single-precision)"))
  ;[1 1 1] Y Movement
  (if (!= AxisValue 0.0)
    (if (not (or (`/Game/Widgets/HUD.In_Conversation` (`self.HUDReference`)) (`self.Pause`)))
      (bind _output_get (set `self.TemporaryPosition` (`self.K2_GetActorLocation`)))
      (`self.K2_SetActorLocation` (+ _output_get (`KismetMathLibrary.MakeVector` 0.0 (* AxisValue (`self.Speed`)))) true))))

(event `InputAction|Sprint`
  (params (Key :type "Key Structure"))
  (bind _speed (`self.Speed`))
  (bind _sprintmultiplier (`self.SprintMultiplier`))
  ;[1 1 1] Sprint Action
  (:`Pressed`
    (set `self.Speed` (* _speed _sprintmultiplier)))
  (:`Released`
    (set `self.Speed` (/ _speed _sprintmultiplier))))

(fn `Check if Standing on Class Member`
  (params (ActorClass :type "Actor Class Reference"))
  (returns (IsStanding :type Boolean))
  (bind _outactors (`GameplayStatics.GetAllActorsOfClass` ActorClass))
  (for _array_element _outactors
    (if (== (`self.K2_GetActorLocation` self) (`self.K2_GetActorLocation` _array_element) :`ErrorTolerance` 50.0)
      (`|ExecutionSequence`
        (:`then_0`
          (break))
        (:`then_1`
          (return true)))))
  (return false))

(fn `Compare Actor Locations`
  (params (FirstActor :type "Actor Object Reference") (SecondActor :type "Actor Object Reference"))
  (returns (NewParam :type Boolean))
  (return (== (`self.K2_GetActorLocation` FirstActor) (`self.K2_GetActorLocation` SecondActor) :`ErrorTolerance` 50.0)))

(fn `Conversation Give Clue`
  (params (HudRef :type "/Game/Widgets/HUD Object Reference (by ref)") (Wanted :type "Integer (by ref)") (QStage :type "Integer (by ref)") (Actor :type "/Game/BP_Directory/NPC_BP Object Reference (by ref)"))
  (for _index (range 4)
    (if (== QStage _index)
      (set `/Game/Widgets/HUD.TextShow` (+ (* Wanted 10) _index) HudRef)
      (set `/Game/BP_Directory/NPC_BP.QStage` (+ QStage 1) Actor)
      (return)))
  (set `/Game/Widgets/HUD.TextShow` (+ (* Wanted 10) 4) HudRef))

(fn `Conversation Good Item`
  (params (HudRef :type "/Game/Widgets/HUD Object Reference (by ref)") (ActorRef :type "/Game/BP_Directory/NPC_BP Object Reference (by ref)") (MyItem :type "Integer (by ref)"))
  (set `/Game/Widgets/HUD.TextShow` (+ (* MyItem 10) 5) HudRef)
  (set `/Game/Widgets/HUD.Item_Carried` 0 HudRef)
  (set `/Game/BP_Directory/NPC_BP.Item_Want` 0 ActorRef))

(fn `Conversation Progressing`
  (params (ItemCarriedReference :type "Integer (by ref)") (ItemWantReference :type "Integer (by ref)") (ConversationStage :type "Integer (by ref)") (HUDPassReference :type "/Game/Widgets/HUD Object Reference (by ref)") (ActorPassRef :type "/Game/BP_Directory/NPC_BP Object Reference (by ref)"))
  (locals (ItemCarried :type Integer) (ItemWant :type Integer) (ConversationStageReference :type Integer) (HudRef :type "/Game/Widgets/HUD Object Reference") (ActorRef :type "/Game/BP_Directory/NPC_BP Object Reference"))
  (set `local.ItemCarried` ItemCarriedReference)
  (set `local.ItemWant` ItemWantReference)
  (set `local.ConversationStageReference` ConversationStage)
  (set `local.HudRef` HUDPassReference)
  (bind _output_get (set `local.ActorRef` ActorPassRef))
  (set `/Game/Widgets/HUD.NPC_Face` (`/Game/BP_Directory/NPC_BP.Identity` _output_get) HUDPassReference)
  (if (== (`local.ItemCarried`) (`local.ItemWant`))
    (`self.Conversation Good Item` (`local.HudRef`) (`local.ActorRef`) (`local.ItemWant`))
    (else
      (`self.Conversation Give Clue` (`local.HudRef`) (`local.ItemWant`) (`local.ConversationStageReference`) (`local.ActorRef`)))))

(fn `DropItem`
  (`|SpawnActorFromClass` "/Game/BP_Directory/Item_BP.Item_BP_C" (`KismetMathLibrary.MakeTransform` (`self.K2_GetActorLocation` self)) "Undefined" "OverrideRootScale" null (`/Game/Widgets/HUD.Item_Carried` (`self.HUDReference`)) null)
  (set `/Game/Widgets/HUD.Item_Carried` 0 (`self.HUDReference`)))

(fn `EndCoversation`
  (set `/Game/Widgets/HUD.In_Conversation` false (`self.HUDReference`))
  (bind _outactors (`GameplayStatics.GetAllActorsOfClass` "/Game/BP_Directory/NPC_BP.NPC_BP_C"))
  (for (_array_element _array_index) _outactors
    (if (== (`self.K2_GetActorLocation` self) (`self.K2_GetActorLocation` _array_element) :`ErrorTolerance` 50.0)
      (bind _output (`|GetArrayItem` _outactors _array_index))
      (if (== (`/Game/BP_Directory/NPC_BP.Item_Want` _output) 0)
        (`self.K2_DestroyActor` _output)
        (bind _output_get (set `self.KillCounter` (+ (`self.KillCounter`) 1)))
        (`KismetSystemLibrary.PrintString` (`KismetStringLibrary.Conv_IntToString` _output_get))))))

(fn `PickupItem`
  (bind _outactors (`GameplayStatics.GetAllActorsOfClass` "/Game/BP_Directory/Item_BP.Item_BP_C"))
  (for (_array_element _array_index) _outactors
    (if (== (`self.K2_GetActorLocation` self) (`self.K2_GetActorLocation` _array_element) :`ErrorTolerance` 25.0)
      (bind _output (`|GetArrayItem` _outactors _array_index))
      (set `/Game/Widgets/HUD.Item_Carried` (`/Game/BP_Directory/Item_BP.Index` _output) (`self.HUDReference`))
      (`self.K2_DestroyActor` _output)
      (break))))

(fn `StartConversation`
  (bind _hudreference (`self.HUDReference`))
  (bind _outactors (`GameplayStatics.GetAllActorsOfClass` "/Game/BP_Directory/NPC_BP.NPC_BP_C"))
  (for _array_element _outactors
    (if (== (`self.K2_GetActorLocation` self) (`self.K2_GetActorLocation` _array_element) :`ErrorTolerance` 50.0)
      (`self.Conversation Progressing` (`/Game/Widgets/HUD.Item_Carried` _hudreference) (`/Game/BP_Directory/NPC_BP.Item_Want` _array_element) (`/Game/BP_Directory/NPC_BP.QStage` _array_element) _hudreference _array_element))))

(fn `SwapItem`
  (params (ItemCarried :type "Integer (by ref)"))
  (locals (TempCarriedItem :type Integer))
  (bind _output_get (set `local.TempCarriedItem` ItemCarried))
  (bind _outactors (`GameplayStatics.GetAllActorsOfClass` "/Game/BP_Directory/Item_BP.Item_BP_C"))
  (for (_array_element _array_index) _outactors
    (if (== (`self.K2_GetActorLocation` self) (`self.K2_GetActorLocation` _array_element) :`ErrorTolerance` 100.0)
      (bind _output (`|GetArrayItem` _outactors _array_index))
      (bind _output_get_2 (set `/Game/Widgets/HUD.Item_Carried` (`/Game/BP_Directory/Item_BP.Index` _output) (`self.HUDReference`)))
      (`self.K2_DestroyActor` _output)
      (`|SpawnActorFromClass` "/Game/BP_Directory/Item_BP.Item_BP_C" (`KismetMathLibrary.MakeTransform` (`self.K2_GetActorLocation` self)) "Undefined" "OverrideRootScale" null _output_get null)
      (set `/Game/Widgets/HUD.Item_Carried` _output_get_2 (`self.HUDReference`)))))

(fn `UserConstructionScript`)

(fn `VictoryCondition`
  (`GameplayStatics.OpenLevel` "EndGame"))